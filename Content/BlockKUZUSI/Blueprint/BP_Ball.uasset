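; Ball actor for a block-breaker game that registers with BallManager on spawn and unregisters when destroyed.
; Its launch vector combines up with a random left or right, and a looping timer drives movement, apparently through swept world offsets rather than physics.
; Hits mirror that vector on the surface normal within the YZ plane and play a click.
; Block hits destroy the struck item and randomize the ball's emissive color.
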(event `self.ReceiveBeginPlay`
  ;[0 0 0] - ゲーム開始時にBallManagerクラスのAddBall関数をコールする
  ;  - Call the AddBall function in the BallManager class at the start of the game
  (`/Game/BlockKUZUSI/Blueprint/BP_BallManager.AddBall` (`self.BallManager`) self))

(event `CE_AddForceToBallLoop`
  (bind _returnvalue (* (`self.BallSpeed`) (`GameplayStatics.GetWorldDeltaSeconds`)))
  ;[0 0 0] - BallにForceを加える処理/この処理の前にSetRandomVector関数が呼ばれる
  ;  - The process of adding force to a ball/Before this process, the SetRandomVector function is called
  (set `self.DrivingForce` (+ (* (`self.GetActorUpVector`) _returnvalue) (* (`self.RandomVector`) _returnvalue)))
  (bind _returnvalue_2 (`KismetSystemLibrary.K2_SetTimerDelegate` (`|CreateDelegate` :!event `AddForceToBall`) (`GameplayStatics.GetWorldDeltaSeconds`) true))
  (set `self.AddForceToBallLoopTimer` _returnvalue_2))

(event `self.BallMesh.OnComponentHit`
  (params (HitComponent :type "PrimitiveComponent Object Reference") (OtherActor :type "Actor Object Reference") (OtherComp :type "PrimitiveComponent Object Reference") (NormalImpulse :type "Vector Structure") (Hit :type "HitResult Structure (by ref)"))
  (bind (_returnvalue_x _returnvalue_y _returnvalue_z) (`KismetMathLibrary.BreakVector` (`KismetMathLibrary.MirrorVectorByNormal` (`self.DrivingForce`) Hit_ImpactNormal)))
  ;[0 0 0] - BallがHitした時のイベント
  ;  - The event when the ball is hit.
  (set `self.DrivingForce` (`KismetMathLibrary.MakeVector` 0.0 _returnvalue_y _returnvalue_z))
  (`GameplayStatics.SpawnSoundAtLocation` "/Engine/VREditor/Sounds/VR_click2_Cue.VR_click2_Cue" (`self.K2_GetActorLocation`) (struct) 0.5 1.0 0.0 null null)
  (bind _asbp_block (cast `/Game/BlockKUZUSI/Blueprint/BP_Block` OtherActor)) ; もし、ボールにヒットしたら
  (`/Game/BlockKUZUSI/Blueprint/BP_Block.DestroyBlock` _asbp_block Hit_HitItem)
  (`self.SetRandomBallColor`))

(fn `AddForceToBall`
  ;[0 0 0] - DrivingForce変数を元にBallに持続的なForceを与える
  ;  - Giving the ball a persistent force based on the DrivingForce variable
  (`SceneComponent.K2_AddWorldOffset` (`self.BallMesh`) (`self.DrivingForce`) true false))

(fn `DestroyBall`
  ;[0 0 0] - Killzoneに入ったらBallManagerのRemoveBall関数をコールし、ボールを削除する
  ;  - When you enter Killzone, call the BallManager's RemoveBall function and remove the ball
  (`GameplayStatics.SpawnSound2D` "/Engine/EditorSounds/Notifications/CompileFailed_Cue.CompileFailed_Cue" 1.0 1.0 0.0 null)
  (`/Game/BlockKUZUSI/Blueprint/BP_BallManager.RemoveBall` (`self.BallManager`) self)
  (`self.K2_DestroyActor`))

(fn `SetRandomBallColor`
  (bind _colors (`self.Colors`))
  ;[0 0 0] - Colors配列からランダムな色を決定する
  ;  - Determine a random color from the Colors array
  (set `self.NewColor` (`|GetArrayItem` _colors (`KismetMathLibrary.RandomIntegerInRange` 0 (- (`KismetArrayLibrary.Array_Length` _colors) 1))))
  (`MaterialInstanceDynamic.SetVectorParameterValue` (`self.MI`) "EmissiveColor" (`self.NewColor`)))

(fn `SetRandomVector`
  ;[0 0 0] - BallがSpawn時に呼ばれる,右か左どちらかに飛ばされる
  ;  - Called when the ball is spawned, it is sent to the right or left
  (set `self.RandomVector` (* (`self.GetActorRightVector`) (`KismetMathLibrary.SelectFloat` 1.0 -1.0 (`KismetMathLibrary.RandomBoolWithWeight` 0.5)))))

(fn `UserConstructionScript`
  (bind _returnvalue (`PrimitiveComponent.CreateDynamicMaterialInstance` (`self.BallMesh`) 0 null "None"))
  (set `self.MI` _returnvalue))
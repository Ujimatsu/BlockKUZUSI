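; BP_BallManager keeps track of the balls in play in the block-breaker game.
; It holds them in a Balls array, adding each ball uniquely and removing it on request.
; Query functions report whether any ball exists, by checking that index 0 is valid, and how many there are, from the array length.
; It only does bookkeeping and does not spawn or destroy balls itself.
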(fn `AddBall`
  (params (NewBall :type "/Game/BlockKUZUSI/Blueprint/BP_Ball Object Reference (by ref)"))
  ;[0 0 0] - Ball配列に新しいBallクラスをAddする
  ;  - Add a new ball class to the ball array
  (`KismetArrayLibrary.Array_AddUnique` (`self.Balls`) NewBall))

(fn `DoesBallExist`
  (returns (ReturnValue :type Boolean))
  ;[0 0 0] - ボールがLevel上にあるかチェックする
  ;  - Check if the ball is on Level
  (return (`KismetArrayLibrary.Array_IsValidIndex` (`self.Balls`))))

(fn `GetNumOfBalls`
  (returns (ReturnValue :type Integer))
  ;[0 0 0] - Level上にあるボールの個数をチェック
  ;  - Check the number of balls on the Level
  (return (`KismetArrayLibrary.Array_Length` (`self.Balls`))))

(fn `RemoveBall`
  (params (RemoveBall :type "/Game/BlockKUZUSI/Blueprint/BP_Ball Object Reference (by ref)"))
  ;[0 0 0] - Balls配列からBallを削除
  ;  - Remove ball from the Balls array
  (`KismetArrayLibrary.Array_RemoveItem` (`self.Balls`) RemoveBall))

(fn `UserConstructionScript`)
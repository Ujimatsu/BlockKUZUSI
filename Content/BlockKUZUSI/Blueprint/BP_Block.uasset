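; BP_Block is the breakable block wall of a breakout-style game, laid out as a grid of instances in one InstancedStaticMesh.
; The construction script builds the grid from horizontal and vertical counts, spacing instances by mesh bounds plus a small gap.
; DestroyBlock removes the given instance, occasionally spawning an extra launched ball there using the BallManager cached at BeginPlay.
; When no instances remain, it shows the game-clear widget.
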(event `self.ReceiveBeginPlay`
  ;[0 0 0] - ゲーム開始時にBallManagerクラスをゲットしリファレンスを保持
  ;  - Get the BallManager class at the start of the game and keep the reference
  (bind _outactors (`GameplayStatics.GetAllActorsOfClass` "/Game/BlockKUZUSI/Blueprint/BP_BallManager.BP_BallManager_C"))
  (if (`KismetArrayLibrary.Array_IsValidIndex` _outactors)
    (set `self.BallManager` (`|GetArrayItem` _outactors))))

(fn `DestroyBlock`
  (params (InstanceIndex :type Integer))
  ;[0 0 0] - Blockの破壊処理,InstancedStaticMeshで表現しているのでBlockの破壊はRemoveInstance関数で行う
  ;  - Block Destruction Process,The block is expressed in InstancedStaticMesh, so the block is destroyed by the RemoveInstance function
  (if (`KismetMathLibrary.RandomBoolWithWeight` 0.05)
    (bind _returnvalue (`|SpawnActorFromClass` "/Game/BlockKUZUSI/Blueprint/BP_Ball.BP_Ball_C" (`InstancedStaticMeshComponent.GetInstanceTransform` (`self.BlockMesh`) InstanceIndex true) "AlwaysSpawn" "OverrideRootScale" null (`self.BallManager`) null))
    (`/Game/BlockKUZUSI/Blueprint/BP_Ball.SetRandomVector` _returnvalue)
    (`/Game/BlockKUZUSI/Blueprint/BP_Ball.CE_AddForceToBallLoop` _returnvalue))
  (`InstancedStaticMeshComponent.RemoveInstance` (`self.BlockMesh`) (`local.InstanceIndex`))
  (if (<= (`InstancedStaticMeshComponent.GetInstanceCount` (`self.BlockMesh`)) 0)
    (bind _returnvalue_2 (`|CreateWidget` "/Game/BlockKUZUSI/Blueprint/WBP_GameClear.WBP_GameClear_C"))
    (`UserWidget.AddToViewport` _returnvalue_2 0)))

(fn `UserConstructionScript`
  (bind (_returnvalue_x _returnvalue_y _returnvalue_z) (`KismetMathLibrary.BreakVector` (* (`.Max` (`StaticMeshComponent.GetLocalBounds` (`self.BlockMesh`))) 2.0)))
  ;[0 0 0] - InstancedStaticMeshの生成処理
  ;  - InstancedStaticMesh generation logic
  (for _index (range 1 (+ (`self.HorizontalLoop`) 1))
    (for _index_2 (range 1 (+ (`self.VerticalLoop`) 1))
      (`InstancedStaticMeshComponent.AddInstance` (`self.BlockMesh`) (`KismetMathLibrary.MakeTransform` (`KismetMathLibrary.MakeVector` 0.0 (* _index (* _returnvalue_y 1.02)) (* _index_2 (* _returnvalue_z 1.02))))))))
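; BP_PlayerBar is the player's paddle in a block-breaker game, moving sideways and launching the ball.
; Axis input slides the bar mesh along the actor's right vector with sweep, scaled by speed and delta time.
; The spawn action asks the level's BP_BallManager whether a ball exists, and if none does, spawns one above the bar with a random direction.
; Ball hits play a Flash timeline that drives HitAlpha on the bar's dynamic material.
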(event `self.ReceiveBeginPlay`
  ;[0 0 0] - ゲーム開始時にBallManagerクラスをゲットしリファレンスを保持
  ;  - Get the BallManager class at the start of the game and keep the reference
  (bind _outactors (`GameplayStatics.GetAllActorsOfClass` "/Game/BlockKUZUSI/Blueprint/BP_BallManager.BP_BallManager_C"))
  (if (`KismetArrayLibrary.Array_IsValidIndex` _outactors)
    (set `self.BallManager` (`|GetArrayItem` _outactors))))

(event `InputAxis|MoveBar`
  (params (AxisValue :type "Float (single-precision)"))
  ;[0 0 0] - バーを動かす処理
  ;  - The process of moving the bar
  (`SceneComponent.K2_AddWorldOffset` (`self.BarMesh`) (* (* (`self.GetActorRightVector`) (`KismetMathLibrary.FClamp` AxisValue -1.0)) (* (`self.BarMoveSpeed`) (`GameplayStatics.GetWorldDeltaSeconds`))) true false))

(event `self.BarMesh.OnComponentHit`
  (params (HitComponent :type "PrimitiveComponent Object Reference") (OtherActor :type "Actor Object Reference") (OtherComp :type "PrimitiveComponent Object Reference") (NormalImpulse :type "Vector Structure") (Hit :type "HitResult Structure (by ref)"))
  ;[0 0 0] - バーにボールがヒットした時の発光エフェクト
  ;  - The lighting effect when the ball hits the bar.
  (cast `/Game/BlockKUZUSI/Blueprint/BP_Ball` OtherActor)
  (bind (_direction _alpha) (`Timeline|Flash` :!via `PlayFromStart`)
    (:`Update`
      (`MaterialInstanceDynamic.SetScalarParameterValue` (`self.MI_Bar`) "HitAlpha" _alpha))))

(event `InputAction|SpawnBall`
  (params (Key :type "Key Structure"))
  (bind _barmesh (`self.BarMesh`))
  ;[0 0 0] - ボールのSpawn処理
  ;  - Ball spawn logic
  (:`Pressed`
    (if (not (`/Game/BlockKUZUSI/Blueprint/BP_BallManager.DoesBallExist` (`self.BallManager`)))
      (bind _returnvalue (`|SpawnActorFromClass` "/Game/BlockKUZUSI/Blueprint/BP_Ball.BP_Ball_C" (`KismetMathLibrary.MakeTransform` (+ (`SceneComponent.K2_GetComponentLocation` _barmesh) (* (`SceneComponent.GetUpVector` _barmesh) 30.0))) "AlwaysSpawn" "OverrideRootScale" null (`self.BallManager`) null))
      (`/Game/BlockKUZUSI/Blueprint/BP_Ball.SetRandomVector` _returnvalue)
      (`/Game/BlockKUZUSI/Blueprint/BP_Ball.CE_AddForceToBallLoop` _returnvalue))))

(fn `UserConstructionScript`
  (bind _returnvalue (`PrimitiveComponent.CreateDynamicMaterialInstance` (`self.BarMesh`) 0 null "None"))
  (set `self.MI_Bar` _returnvalue))